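; Game instance blueprint that manages saved level and ability progress and opens the splash and hotbar widgets.
; Init checks the default slot, creating a BP_SaveGame if none exists; the load branch never assigns its result to SaveGame.
; Save events update completion arrays by index and write immediately, while getters expose both arrays.
; When enabled, the splash appears after a one-tick delay with sound and UI-only input; InitHotbar is a separate event.
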(event Custom|SaveLevelStatus
  (params (Level :type Integer) (Completed :type Boolean))
  (Utilities|Array|SetArrayElem (Variables|/Game/Blueprints/BP_SaveGame.BP_SaveGame_C|GetCompletedLevels (Variables|Default|GetSaveGame)) Level Completed)
  (SaveGame|SaveGametoSlot (Variables|Default|GetSaveGame) (Variables|Default|GetDefaultSlotName)))

(event Custom|SaveAbilityStatus
  (params (Level :type Integer) (Completed :type Boolean))
  (Utilities|Array|SetArrayElem (Variables|/Game/Blueprints/BP_SaveGame.BP_SaveGame_C|GetAcquiredAbilities (Variables|Default|GetSaveGame)) Level Completed)
  (SaveGame|SaveGametoSlot (Variables|Default|GetSaveGame) (Variables|Default|GetDefaultSlotName)))

(event Custom|InitSaveSystem
  (bind _returnvalue (SaveGame|DoesSaveGameExist (Variables|Default|GetDefaultSlotName)))
  (if _returnvalue
    (SaveGame|LoadGamefromSlot (Variables|Default|GetDefaultSlotName))
    (else
      (bind _returnvalue_2 (SaveGame|CreateSaveGameObject "/Game/Blueprints/BP_SaveGame.BP_SaveGame_C"))
      (Variables|Default|SetSaveGame _returnvalue_2))))

(event Custom|ShowSplashScreen
  (bind _returnvalue (Game|GetPlayerController 0))
  (if (Variables|Default|GetSplash)
    (Utilities|FlowControl|DelayUntilNextTick)
    (bind _returnvalue_2 (UserInterface|CreateWidget "/Game/Blueprints/Widgets/WBP_Splash.WBP_Splash_C" (Game|GetPlayerController 0)))
    (UserInterface|Viewport|AddtoPlayerScreen _returnvalue_2)
    (Audio|PlaySound2D "/Game/Assets/SFX/SupersonicPalto.SupersonicPalto" 1.0 1.0 0.0 0 0)
    (Input|SetInputModeUIOnly _returnvalue _returnvalue_2 "DoNotLock" false)
    (Variables|/Script/Engine.PlayerController|SetbShowMouseCursor _returnvalue true)))

(event Custom|InitHotbar
  (Utilities|FlowControl|DelayUntilNextTick)
  (bind _returnvalue (UserInterface|CreateWidget "/Game/Blueprints/Widgets/WBP_Hotbar.WBP_Hotbar_C" (Game|GetPlayerController 0)))
  (UserInterface|Viewport|AddtoViewport _returnvalue 0))

(event EventInit
  (CallFunction|InitSaveSystem)
  (CallFunction|ShowSplashScreen))

(fn GetCompletedLevels
  (return (Variables|/Game/Blueprints/BP_SaveGame.BP_SaveGame_C|GetCompletedLevels (Variables|Default|GetSaveGame))))

(fn GetAcquiredAbilities
  (return (Variables|/Game/Blueprints/BP_SaveGame.BP_SaveGame_C|GetAcquiredAbilities (Variables|Default|GetSaveGame))))