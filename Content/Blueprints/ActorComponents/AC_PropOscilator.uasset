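; Actor component that oscillates its owning actor back and forth from its starting location along any combination of world X, Y and Z.
; If active at BeginPlay, it runs TFAnimation on a looping timer instead of Tick.
; Each step ping-pongs an alpha between 0 and 1, with CycleDurationInSeconds covering one direction.
; A float curve maps that alpha, scaled by MovementRange, to the offset on each enabled axis.
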(event EventBeginPlay
  (Variables|Default|SetOwnerActor (Components|GetOwner))
  (CallFunction|SetOwnerStartingLocation)
  (if (Variables|Default|GetbOscilationActive)
    (Utilities|Time|SetTimerbyFunctionName 0 "TFAnimation" (Variables|Default|GetAnimationRefresh%20time) true)))

(event EventTick
  (params (DeltaSeconds :type Float%20%28single-precision%29)))

(fn TFAnimation
  (bind _ownerstartinglocation (Variables|Default|GetOwnerStartingLocation))
  (bind _ownerstartinglocation_2 (Variables|Default|GetOwnerStartingLocation))
  (bind _owneractor (Variables|Default|GetOwnerActor))
  (bind _returnvalue (Transformation|GetActorLocation _owneractor))
  (Utilities|FlowControl|Sequence
    (:then_0
      ;[1 1 1] Comment
      (if (<= (Variables|Default|GetAnimationAlpha) 0.0)
        (Variables|Default|SetbAnimationAlphaGoingUp true)
        (Variables|Default|SetAnimationAlpha 0.0)
        (elif (>= (Variables|Default|GetAnimationAlpha) 1.0)
          (Variables|Default|SetbAnimationAlphaGoingUp false)
          (Variables|Default|SetAnimationAlpha 1.0))))
    (:then_1
      (if (Variables|Default|GetbAnimationAlphaGoingUp)
        ;[1 1 1] Comment
        (Variables|Default|SetAnimationAlpha (+ (Variables|Default|GetAnimationAlpha) (* (/ 1.0 (Variables|Default|GetCycleDurationInSeconds)) (Variables|Default|GetAnimationRefresh%20time))))
        (else
          ;[1 1 1] Comment
          (Variables|Default|SetAnimationAlpha (- (Variables|Default|GetAnimationAlpha) (* (/ 1.0 (Variables|Default|GetCycleDurationInSeconds)) (Variables|Default|GetAnimationRefresh%20time)))))))
    (:then_2
      (Utilities|FlowControl|Sequence
        (:then_0
          ;[1 1 1] x
          (if (Variables|Default|GetbAffectXAxis)
            (Transformation|SetActorLocation (Variables|Default|GetOwnerActor) (Math|Vector|MakeVector (+ (.x _ownerstartinglocation) (* (Math|Curves|GetFloatValue (Variables|Default|GetCurveFloat) (Variables|Default|GetAnimationAlpha)) (Variables|Default|GetMovementRange))) (.y _ownerstartinglocation) (.z _ownerstartinglocation)) false false)))
        (:then_1
          ;[1 1 1] y
          (if (Variables|Default|GetbAffectYAxis)
            (Transformation|SetActorLocation (Variables|Default|GetOwnerActor) (Math|Vector|MakeVector (.x (Transformation|GetActorLocation (Variables|Default|GetOwnerActor))) (+ (.y _ownerstartinglocation_2) (* (Math|Curves|GetFloatValue (Variables|Default|GetCurveFloat) (Variables|Default|GetAnimationAlpha)) (Variables|Default|GetMovementRange))) (.z _ownerstartinglocation_2)) false false)))
        (:then_2
          ;[1 1 1] z
          (if (Variables|Default|GetbAffectZAxis)
            (Transformation|SetActorLocation (Variables|Default|GetOwnerActor) (Math|Vector|MakeVector (.x _returnvalue) (.y _returnvalue) (+ (.z (Variables|Default|GetOwnerStartingLocation)) (* (Math|Curves|GetFloatValue (Variables|Default|GetCurveFloat) (Variables|Default|GetAnimationAlpha)) (Variables|Default|GetMovementRange)))) false false)))))))

(fn SetOwnerStartingLocation
  (Variables|Default|SetOwnerStartingLocation (Transformation|GetActorLocation (Variables|Default|GetOwnerActor))))